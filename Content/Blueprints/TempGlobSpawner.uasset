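; TempGlobSpawner is a spawner actor that keeps creating GlobTroopBP actors around its own location.
; It spawns an initial batch on BeginPlay, then Tick accumulates a timer and spawns a smaller batch every few seconds.
; SpawnGloob places each troop at a small random positive X/Z offset with the spawner's rotation, always spawning regardless of collision.
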(event `self.ReceiveBeginPlay`
  (for _ (range 6)
    (`self.Spawn Gloob`)))

(event `self.ReceiveTick`
  (params (DeltaSeconds :type "Float (single-precision)"))
  (bind _timer (`self.timer`))
  (set `self.timer` (+ DeltaSeconds _timer))
  (if (> _timer 3.0)
    (set `self.timer` 0.0)
    (for _ (range 3)
      (`self.Spawn Gloob`))))

(event `Spawn Gloob`
  (`|SpawnActorFromClass` "/Game/Blueprints/TroopBPs/GlobTroopBP.GlobTroopBP_C" (`KismetMathLibrary.MakeTransform` (+ (`self.K2_GetActorLocation`) (* (`KismetMathLibrary.MakeVector` (`KismetMathLibrary.RandomFloat`) 0.0 (`KismetMathLibrary.RandomFloat`)) 50.0)) (`self.K2_GetActorRotation`)) "AlwaysSpawn" "MultiplyWithRoot" null null))

(fn `UserConstructionScript`)