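; BP_DefenseBlockBasic is a melee defense unit with cactus attack animation that damages enemies in range.
; Its Attack event switches the sprite to the attack flipbook and applies Damage to the first entry in EnemiesInRange, printing debug messages.
; Tick watches the playback frame and returns the sprite to the melee idle flipbook when the attack reaches its last frame.
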(event `StopAttackAnimation`)

(event `self.ReceiveBeginPlay`)

(event `self.ReceiveTick`
  (params (DeltaSeconds :type "Float (single-precision)"))
  (if (and (== (- (`PaperFlipbook.GetNumFrames` (`PaperFlipbookComponent.GetFlipbook` (`self.Sprite`))) 1) (`PaperFlipbookComponent.GetPlaybackPositionInFrames` (`self.Sprite`))) (== (`PaperFlipbookComponent.GetFlipbook` (`self.Sprite`)) "/Game/Assets/Towers/melee/CactusAttackFlipbook.CactusAttackFlipbook"))
    (`PaperFlipbookComponent.SetFlipbook` (`self.Sprite`) "/Game/Assets/Towers/melee/melee_idle.melee_idle")))

(event `self.Attack`
  (if (> (`KismetArrayLibrary.Array_Length` (`self.EnemiesInRange`)) 0)
    (`KismetSystemLibrary.PrintString` "Attacking")
    (`PaperFlipbookComponent.SetFlipbook` (`self.Sprite`) "/Game/Assets/Towers/melee/CactusAttackFlipbook.CactusAttackFlipbook")
    (`TroopBase.DamageHealth` (`|GetArrayItem` (`self.EnemiesInRange`)) (`self.Damage`))
    (`KismetSystemLibrary.PrintString` "Did damage")))

(fn `UserConstructionScript`)