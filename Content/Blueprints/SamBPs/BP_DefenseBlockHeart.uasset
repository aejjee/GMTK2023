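; BP_DefenseBlockHeart is a defense block that damages every enemy in range when it attacks.
; Attack flashes the sprite pale yellow and calls DamageHealth with Damage on each entry in EnemiesInRange.
; Tick continuously lerps the sprite color toward dark grey, scaled by delta time, so each flash fades out between attacks.
; The graph only consumes EnemiesInRange; it contains no range detection or attack timing.
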(event `self.ReceiveTick`
  (params (DeltaSeconds :type "Float (single-precision)"))
  (`PaperFlipbookComponent.SetSpriteColor` (`self.Sprite`) (`KismetMathLibrary.LinearColorLerp` (`PaperFlipbookComponent.GetSpriteColor` (`self.Sprite`)) (`KismetMathLibrary.MakeColor` 0.25 0.25 0.25) (* DeltaSeconds 2.0))))

(event `self.Attack`
  (bind _enemiesinrange (`self.EnemiesInRange`))
  (`PaperFlipbookComponent.SetSpriteColor` (`self.Sprite`) (struct :`R` 1.0 :`G` 0.92161 :`B` 0.489159 :`A` 1.0))
  (for (_ _array_index) _enemiesinrange
    (`TroopBase.DamageHealth` (`|GetArrayItem` _enemiesinrange _array_index) (`self.Damage`))))

(fn `UserConstructionScript`)