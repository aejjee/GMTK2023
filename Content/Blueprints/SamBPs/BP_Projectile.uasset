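; BP_Projectile is a homing projectile that damages troops and then destroys itself.
; Each Tick compares its distance to the homing target's owner against the Sphere radius, treating proximity as a hit alongside the regular Hit event.
; Both paths feed ApplyDamageAndDestroy, which calls DamageHealth on a TroopBase before destroying the projectile.
; Defense blocks leave it alive and undamaged, while any other actor destroys it without damage.
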(event `self.ReceiveActorBeginOverlap`
  (params (OtherActor :type "Actor Object Reference")))

(event `self.ReceiveTick`
  (params (DeltaSeconds :type "Float (single-precision)"))
  (bind _returnvalue (`ActorComponent.GetOwner` (`ProjectileMovementComponent.HomingTargetComponent` (`self.ProjectileMovement`))))
  (if (< (`KismetMathLibrary.VSize` (- (`self.K2_GetActorLocation` _returnvalue) (`self.K2_GetActorLocation`))) (`SphereComponent.GetScaledSphereRadius` (`self.Sphere`)))
    (`self.Apply Damage And Destroy` _returnvalue)))

(event `self.ReceiveHit`
  (params (MyComp :type "PrimitiveComponent Object Reference") (Other :type "Actor Object Reference") (OtherComp :type "PrimitiveComponent Object Reference") (bSelfMoved :type Boolean) (HitLocation :type "Vector Structure") (HitNormal :type "Vector Structure") (NormalImpulse :type "Vector Structure") (Hit :type "HitResult Structure (by ref)"))
  (`self.Apply Damage And Destroy` Other))

(event `self.Sphere.OnComponentBeginOverlap`
  (params (OverlappedComponent :type "PrimitiveComponent Object Reference") (OtherActor :type "Actor Object Reference") (OtherComp :type "PrimitiveComponent Object Reference") (OtherBodyIndex :type Integer) (bFromSweep :type Boolean) (SweepResult :type "HitResult Structure (by ref)")))

(event `Apply Damage And Destroy`
  (params (Actor :type "Actor Object Reference"))
  (bind _astroop_base (cast `TroopBase` Actor)
    (:`then`
      (`TroopBase.DamageHealth` _astroop_base (`self.Damage`))
      (`self.K2_DestroyActor`))
    (:`CastFailed`
      (cast `DefenseBlockBase` Actor
        (:`CastFailed`
          (`self.K2_DestroyActor`))))))

(fn `UserConstructionScript`)