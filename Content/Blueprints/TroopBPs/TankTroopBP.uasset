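; Tank troop Blueprint that handles switching its Paper2D sprite between a default and an attack flipbook, both using Glob assets.
; BeginPlay stores the attack flipbook, and PlayAttackAnimation sets a playing flag and applies it to the sprite.
; Tick restores the default flipbook whenever the flag is set and the current flipbook reaches its last frame; the flag is never cleared here.
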(event `self.ReceiveBeginPlay`
  (set `self.attackAnimation` "/Game/Assets/Enemies/basic_enemy/basic_enemy_attack/GlobAttackFlipbook.GlobAttackFlipbook"))

(event `self.ReceiveTick`
  (params (DeltaSeconds :type "Float (single-precision)"))
  (bind _sprite (`self.Sprite`))
  (if (and (`self.attackPlaying`) (== (- (`PaperFlipbook.GetNumFrames` (`PaperFlipbookComponent.GetFlipbook` _sprite)) 1) (`PaperFlipbookComponent.GetPlaybackPositionInFrames` _sprite)))
    (`PaperFlipbookComponent.SetFlipbook` (`self.Sprite`) "/Game/Assets/Enemies/basic_enemy/basic_enemy_walk/GlobFlipbook.GlobFlipbook")))

(event `self.PlayAttackAnimation`
  (set `self.attackPlaying` true)
  (`PaperFlipbookComponent.SetFlipbook` (`self.Sprite`) (`self.attackAnimation`)))

(fn `UserConstructionScript`)