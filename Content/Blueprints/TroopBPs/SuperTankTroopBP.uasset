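; Super tank troop Blueprint with a flipbook sprite and a widget showing its group number.
; Each Tick, while a flipbook is set, it refreshes that number and turns the widget to face the player camera.
; It also restores the walk flipbook on an attack's last frame if AttackPlaying is set.
; PlayAttackAnimation is empty, and the nodes that start the attack flipbook are disconnected.
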(event `self.ReceiveBeginPlay`)

(event `self.ReceiveTick`
  (params (DeltaSeconds :type "Float (single-precision)"))
  (bind _sprite (`self.Sprite`))
  (bind _returnvalue (`PaperFlipbookComponent.GetFlipbook` _sprite))
  (`/Engine/EditorBlueprintResources/StandardMacros.IsValid` _returnvalue
    (:`Is Valid`
      (if (and (`self.attackPlaying`) (== (- (`PaperFlipbook.GetNumFrames` _returnvalue) 1) (`PaperFlipbookComponent.GetPlaybackPositionInFrames` _sprite)))
        (`PaperFlipbookComponent.SetFlipbook` (`self.Sprite`) "/Game/Assets/Enemies/SuperTankEnemy/Walk/A_SuperTankEnemy_Walk.A_SuperTankEnemy_Walk"))
      (`self.SetGroupWidgetText`)
      (`SceneComponent.K2_SetWorldRotation` (`self.GroupWidget`) (`KismetMathLibrary.Conv_VectorToRotator` (`KismetMathLibrary.Normal` (- (`PlayerCameraManager.GetCameraLocation` (`GameplayStatics.GetPlayerCameraManager` 0)) (`self.K2_GetActorLocation`)))) false false))))

(event `self.PlayAttackAnimation`)

(event `SetGroupWidgetText`
  (bind _asgroup_display_widget (cast `/Game/Blueprints/TroopBPs/GroupDisplayWidget` (`WidgetComponent.GetWidget` (`self.GroupWidget`))))
  (set `TextBlock.Text` (`KismetTextLibrary.Conv_IntToText` (`self.groupNumber`)) (`/Game/Blueprints/TroopBPs/GroupDisplayWidget.GroupNumberText` _asgroup_display_widget)))

(fn `UserConstructionScript`)