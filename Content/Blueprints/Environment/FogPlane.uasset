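; FogPlane is an environment actor that intensifies fog-of-war clouds when the player enters combat mode.
; BeginPlay creates a dynamic fog material instance and resets curvature, offset and speed in a Material Parameter Collection.
; While the player pawn is in CombatMode, Tick lerps all three toward higher values and writes them to the collection, gated only on curvature nearing its target.
; No branch eases the values back when combat ends.
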(event `self.ReceiveBeginPlay`
  (set `self.FogCurvature` 0.5)
  (set `self.FogOffset` 0.0)
  (set `self.FogSpeed` 1.0)
  (bind _returnvalue (`PrimitiveComponent.CreateDynamicMaterialInstance` (`self.e`) 0 "/Game/Materials/FogOfWar.FogOfWar" "None"))
  (set `self.FogMaterial` _returnvalue)
  (`KismetMaterialLibrary.SetScalarParameterValue` "/Game/Materials/FogOfWarCloudCollection.FogOfWarCloudCollection" "FogCurvature" 0.5)
  (`KismetMaterialLibrary.SetScalarParameterValue` "/Game/Materials/FogOfWarCloudCollection.FogOfWarCloudCollection" "FogOffset" 0.0)
  (`KismetMaterialLibrary.SetScalarParameterValue` "/Game/Materials/FogOfWarCloudCollection.FogOfWarCloudCollection" "FogSpeed" 1.0))

(event `self.ReceiveTick`
  (params (DeltaSeconds :type "Float (single-precision)"))
  (bind _asplayer_character (cast `PlayerCharacter` (`GameplayStatics.GetPlayerPawn` 0)))
  (if (`PlayerCharacter.combatMode` _asplayer_character)
    (if (> (`KismetMathLibrary.Abs` (- (`self.FogCurvature`) 3.0)) 0.05)
      (bind _output_get (set `self.FogCurvature` (`KismetMathLibrary.Lerp` (`self.FogCurvature`) 3.0 DeltaSeconds)))
      (`KismetMaterialLibrary.SetScalarParameterValue` "/Game/Materials/FogOfWarCloudCollection.FogOfWarCloudCollection" "FogCurvature" _output_get)
      (bind _output_get_2 (set `self.FogOffset` (`KismetMathLibrary.Lerp` (`self.FogOffset`) 0.5 DeltaSeconds)))
      (`KismetMaterialLibrary.SetScalarParameterValue` "/Game/Materials/FogOfWarCloudCollection.FogOfWarCloudCollection" "FogOffset" _output_get_2)
      (bind _output_get_3 (set `self.FogSpeed` (`KismetMathLibrary.Lerp` (`self.FogSpeed`) 3.0 (* DeltaSeconds 2.0))))
      (`KismetMaterialLibrary.SetScalarParameterValue` "/Game/Materials/FogOfWarCloudCollection.FogOfWarCloudCollection" "FogSpeed" _output_get_3))))

(fn `UserConstructionScript`)